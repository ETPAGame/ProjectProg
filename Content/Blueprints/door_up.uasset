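; Interactive door that slides vertically on the player's CloseInteract event, playing an attenuated door sound each time.
; A FlipFlop alternately plays and reverses the Smooth_operture timeline, which drives the Door's relative height, and toggles the player's HUD interact prompt.
; The Box trigger shows that prompt when a FirstPersonCharacter enters with the timeline at or below halfway, and hides it on exit.
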(event OnComponentBeginOverlap(Box)
  (params (OverlappedComponent :type Primitive%20Component%20Object%20Reference) (OtherActor :type Actor%20Object%20Reference) (OtherComp :type Primitive%20Component%20Object%20Reference) (OtherBodyIndex :type Integer) (bFromSweep :type Boolean) (SweepResult :type Hit%20Result%20Structure%20%28by%20ref%29))
  (if (<= (stale EventCloseInteract _newtrack_0) 0.5)
    (bind _asfirst_person_character (Utilities|Casting|CastToFirstPersonCharacter OtherActor))
    (Variables|/Game/Blueprints/FPHUD.FPHUD_C|SetisInteracting (Variables|/Game/Blueprints/FirstPersonCharacter.FirstPersonCharacter_C|GetFPHUD _asfirst_person_character) true)
    (Default|ToggleInteract (Variables|/Game/Blueprints/FirstPersonCharacter.FirstPersonCharacter_C|GetFPHUD _asfirst_person_character))))

(event OnComponentEndOverlap(Box)
  (params (OverlappedComponent :type Primitive%20Component%20Object%20Reference) (OtherActor :type Actor%20Object%20Reference) (OtherComp :type Primitive%20Component%20Object%20Reference) (OtherBodyIndex :type Integer))
  (bind _asfirst_person_character (Utilities|Casting|CastToFirstPersonCharacter OtherActor))
  (Variables|/Game/Blueprints/FPHUD.FPHUD_C|SetisInteracting (Variables|/Game/Blueprints/FirstPersonCharacter.FirstPersonCharacter_C|GetFPHUD _asfirst_person_character) false)
  (Default|ToggleInteract (Variables|/Game/Blueprints/FirstPersonCharacter.FirstPersonCharacter_C|GetFPHUD _asfirst_person_character)))

(event EventBeginPlay)

(event Collision|EventActorBeginOverlap
  (params (OtherActor :type Actor%20Object%20Reference)))

(event EventTick
  (params (DeltaSeconds :type Float%20%28single-precision%29)))

(event EventCloseInteract
  (params (Player :type First%20Person%20Character%20Object%20Reference))
  (bind _fphud (Variables|/Game/Blueprints/FirstPersonCharacter.FirstPersonCharacter_C|GetFPHUD Player))
  (Audio|PlaySoundatLocation "/Game/Son/porte2_Cue.porte2_Cue" (Transformation|GetWorldLocation (Variables|Default|GetSphere)) "0, 0, 0" 0.5 1.0 0.0 "/Game/Son/attenuationdoor.attenuationdoor" 0 0)
  (Utilities|FlowControl|FlipFlop
    (:A
      (Variables|/Game/Blueprints/FPHUD.FPHUD_C|SetisInteracting _fphud false)
      (Default|ToggleInteract _fphud)
      (bind _newtrack_0 (Timeline|smooth_operture Play)
        (:Update
          (Transformation|SetRelativeLocation (Variables|Default|Getdoor) (Math|Vector|MakeVector -3.4e+02 0.0 (* _newtrack_0 3e+02)) false false))))
    (:B
      (Variables|/Game/Blueprints/FPHUD.FPHUD_C|SetisInteracting _fphud true)
      (Default|ToggleInteract _fphud)
      (Timeline|smooth_operture Reverse))))

(fn ConstructionScript)