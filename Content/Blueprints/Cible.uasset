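; Cible is a laser target whose type sets its material and whether the player's laser, the clone's laser or both must hit it.
; Laser hit events set hit flags and call Dead, which resets them after a retriggerable delay if the requirement is unmet.
; Once satisfied, the target is knocked away by physics, plays a sound, loses its emissive glow, then activates its linked platform and opens its linked door.
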(event Custom|scoring
  (params (Add_score_point :type Integer))
  (bind _output_get (Variables|Default|Settarget_score (+ Add_score_point (Variables|Default|Gettarget_score))))
  (Development|PrintString (Utilities|String|ToString(Integer) _output_get)))

(event Custom|Dead
  (params (A :type Vector))
  (bind _cible (Variables|Default|GetCible))
  (if (Utilities|Select :Index (Variables|Default|GetTypeCible) :Option%200 (Variables|Default|GetPlayerHit?) :Option%201 (Variables|Default|GetCloneHit?) :Option%202 (and (Variables|Default|GetPlayerHit?) (Variables|Default|GetCloneHit?)))
    (Physics|SetSimulatePhysics _cible true)
    (Physics|AddImpulse _cible (* A -5e+01) "None" true)
    (Audio|PlaySoundatLocation "/Game/Son/win.win" (Transformation|GetWorldLocation (Variables|Default|GetCible)) "0, 0, 0" 1.0 1.0 0.0 0 0 0)
    (Rendering|Material|SetScalarParameterValueonMaterials (Variables|Default|GetCible) "Emissive" 0.0)
    (Variables|Default|SetIsDead? true)
    (Utilities|FlowControl|Sequence
      (:then_0
        (bind _platform (Variables|Default|GetPlatform)
          (:then
            (Default|Activation _platform))
          (:else)))
      (:then_1
        (bind _door_connect (Variables|Default|GetDoor_Connect)
          (:then
            (Default|OpenDoor _door_connect))
          (:else))))
    (else
      (Utilities|FlowControl|RetriggerableDelay (Variables|Default|GetDuration))
      (Variables|Default|SetPlayerHit? false)
      (Variables|Default|SetCloneHit? false))))

(event EventBeginPlay
  (switch int (Variables|Default|GetTypeCible)
    (:0
      (Rendering|Material|SetMaterial (Variables|Default|GetCible) 0 "/Game/StarterBundle/ModularSci_Comm/Materials/MI_Trims_C_Red1.MI_Trims_C_Red1"))
    (:1
      (Rendering|Material|SetMaterial (Variables|Default|GetCible) 0 "/Game/StarterBundle/ModularSci_Comm/Materials/MI_Trims_C_blue.MI_Trims_C_blue"))
    (:2
      (Rendering|Material|SetMaterial (Variables|Default|GetCible) 0 "/Game/StarterBundle/ModularSci_Comm/Materials/MI_Trims_C_violet.MI_Trims_C_violet"))))

(event EventInteractLaser
  (params (HitDirection :type Vector :default "0, 0, 0"))
  (if (not (Variables|Default|GetIsDead?))
    (Variables|Default|SetPlayerHit? true)
    (CallFunction|Dead HitDirection)
    (CallFunction|Scoring)
    (Development|PrintString "Hello")))

(event EventInteractLaserClone
  (params (HitDirection :type Vector :default "0, 0, 0"))
  (if (not (Variables|Default|GetIsDead?))
    (Variables|Default|SetCloneHit? true)
    (CallFunction|Dead HitDirection)
    (CallFunction|Scoring)
    (Development|PrintString "Hello")))

(fn ConstructionScript)