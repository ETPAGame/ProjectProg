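; Sliding door Blueprint that raises its Door component with sound and a green indicator light, either permanently or as a brief pulse.
; OpenDoor plays the Smooth_operture timeline to lift the door, then hides the light.
; Impulse.OpenDoor plays Fast_door forward, then in reverse, using a counter to end the cycle.
; A DoOnce blocks retriggering until the door closes and the light turns red.
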(event Custom|Open%20Door
  (bind _pointlight (Variables|Default|GetPointLight))
  (Audio|PlaySoundatLocation "/Game/Son/porte2.porte2" (Transformation|GetWorldLocation (Variables|Default|GetSphere)) "0, 0, 0" 1.0 1.0 0.0 "/Game/Son/attenuationdoor.attenuationdoor" 0 0)
  (Rendering|Components|Light|SetLightColor _pointlight "(R=0.081420,G=1.000000,B=0.000000,A=1.000000)" true)
  (bind _newtrack_0 (Timeline|smooth_operture Play)
    (:Update
      (Transformation|SetRelativeLocation (Variables|Default|Getdoor) (Math|Vector|MakeVector -3.4e+02 0.0 (* _newtrack_0 3e+02)) false false))
    (:Finished
      (Rendering|SetVisibility _pointlight false false))))

(event Custom|Open%20Door%20%28Impulse%29
  (bind _pointlight (Variables|Default|GetPointLight))
  (Utilities|FlowControl|DoOnce false :!label _label
    (:Completed
      (Audio|PlaySoundatLocation "/Game/Son/porte2.porte2" (Transformation|GetWorldLocation (Variables|Default|GetSphere)) "0, 0, 0" 1.0 1.0 0.0 "/Game/Son/attenuationdoor.attenuationdoor" 0 0)
      (Rendering|Components|Light|SetLightColor _pointlight "(R=0.081420,G=1.000000,B=0.000000,A=1.000000)" true)
      (bind _newtrack_0 (Timeline|fast_door Play)
        (:Update
          (Transformation|SetRelativeLocation (Variables|Default|Getdoor) (Math|Vector|MakeVector -3.4e+02 0.0 (* _newtrack_0 3e+02)) false false))
        (:Finished
          (bind _result (Math|Integer|IncrementInt (Variables|Default|GetTransit%20Statut%20%28Impulse%29))
            (:%20%20
              (bind _output_get (Variables|Default|SetTransit%20Statut%20%28Impulse%29 _result))
              (if (< _output_get 2)
                (Timeline|fast_door Reverse)
                (else
                  (Variables|Default|SetTransit%20Statut%20%28Impulse%29 0)
                  (Rendering|Components|Light|SetLightColor _pointlight "(R=1.000000,G=0.000000,B=0.000000,A=1.000000)" true)
                  (goto _label Reset))))))))))

(event EventBeginPlay)

(event Collision|EventActorBeginOverlap
  (params (OtherActor :type Actor%20Object%20Reference)))

(event EventTick
  (params (DeltaSeconds :type Float%20%28single-precision%29)))

(fn ConstructionScript)