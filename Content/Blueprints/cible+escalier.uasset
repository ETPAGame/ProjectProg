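; Laser target that, when shot down, makes a linked staircase mesh (NewVar0) appear for one second.
; Laser and clone-laser hits, each gated by a resettable DoOnce, decrement a displayed hit counter that Tick restores when a timer expires.
; At zero the target falls with physics and its light goes out.
; Stairs are shown and hidden by scaling, then the actor respawns a fresh copy and destroys itself.
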(event Custom|ploup
  (bind _cible (Variables|Default|GetCible))
  (Utilities|FlowControl|DoOnce false) ; enters at Reset
)

(event Custom|Plip
  (bind _cible (Variables|Default|GetCible))
  (Utilities|FlowControl|DoOnce false) ; enters at Reset
)

(event Custom|spawnstairs
  (Transformation|SetRelativeScale3D (Variables|/Script/Engine.StaticMeshActor|GetStaticMeshComponent (Variables|Default|GetNewVar_0)) "2.664000,1.198000,2.748000")
  (Utilities|FlowControl|Delay 1.0)
  (CallFunction|Unspawn)
  (bind _returnvalue (Game|SpawnActorfromClass "cible+escalier_C" (Transformation|GetActorTransform self) "Undefined" 0 0))
  (Variables|cible+escalier_C|SetPVBase _returnvalue (Variables|Default|GetPVBase))
  (Variables|cible+escalier_C|SetNewVar_0 _returnvalue (Variables|Default|GetNewVar_0))
  (Actor|DestroyActor))

(event Custom|Unspawn
  (Transformation|SetRelativeScale3D (Variables|/Script/Engine.StaticMeshActor|GetStaticMeshComponent (Variables|Default|GetNewVar_0)) "0, 0, 0"))

(event EventBeginPlay
  (CallFunction|Unspawn)
  (bind _output_get (Variables|Default|SetPoint%20de%20vie (Variables|Default|GetPVBase)))
  (Rendering|Components|TextRender|SetText (Variables|Default|GetTextRender) (Utilities|Text|ToText(Integer) _output_get))
  (Rendering|Components|Light|SetLightColor (Variables|Default|GetPointLight) "(R=0.682292,G=0.032017,B=0.000000,A=1.000000)" true)
  (Variables|Default|SetTimer (Variables|Default|GetTimer%20Base)))

(event Collision|EventActorBeginOverlap
  (params (OtherActor :type Actor%20Object%20Reference)))

(event EventTick
  (params (DeltaSeconds :type Float%20%28single-precision%29))
  (if (and (!= (Variables|Default|GetPoint%20de%20vie) (Variables|Default|GetPVBase)) (> (Variables|Default|GetPoint%20de%20vie) 0))
    (bind _output_get (Variables|Default|SetTimer (- (Variables|Default|GetTimer) DeltaSeconds)))
    (if (<= _output_get 0.0)
      (bind _output_get_2 (Variables|Default|SetPoint%20de%20vie (Variables|Default|GetPVBase)))
      (Variables|Default|SetTimer (Variables|Default|GetTimer%20Base))
      (Rendering|Components|TextRender|SetText (Variables|Default|GetTextRender) (Utilities|Text|ToText(Integer) _output_get_2)))))

(event EventInteractLaser
  (params (HitDirection :type Vector :default "0, 0, 0"))
  (bind _cible (Variables|Default|GetCible))
  (Utilities|FlowControl|DoOnce false
    (:Completed
      (if (> (Variables|Default|GetPoint%20de%20vie) 0)
        (Variables|Default|SetPoint%20de%20vie (- (Variables|Default|GetPoint%20de%20vie) 1))
        (Rendering|Components|TextRender|SetText (Variables|Default|GetTextRender) (Utilities|Text|ToText(Integer) (Variables|Default|GetPoint%20de%20vie)))
        (if (== (Variables|Default|GetPoint%20de%20vie) 0)
          (Physics|SetSimulatePhysics _cible true)
          (Physics|AddImpulse _cible (* HitDirection -5e+01) "None" true)
          (Audio|PlaySoundatLocation "/Game/Son/win.win" (Transformation|GetWorldLocation (Variables|Default|GetPied)) "0, 0, 0" 1.0 1.0 0.0 0 0 0)
          (Rendering|Components|Light|SetIntensity (Variables|Default|GetPointLight) 0.0)
          (CallFunction|Spawnstairs))))))

(event EventInteractLaserClone
  (bind _cible (Variables|Default|GetCible))
  (Development|PrintString "Hello")
  (Utilities|FlowControl|DoOnce false
    (:Completed
      (if (> (Variables|Default|GetPoint%20de%20vie) 0)
        (Variables|Default|SetPoint%20de%20vie (- (Variables|Default|GetPoint%20de%20vie) 1))
        (Rendering|Components|TextRender|SetText (Variables|Default|GetTextRender) (Utilities|Text|ToText(Integer) (Variables|Default|GetPoint%20de%20vie)))
        (if (== (Variables|Default|GetPoint%20de%20vie) 0)
          (Physics|SetSimulatePhysics _cible true)
          (Physics|AddImpulse _cible (* "0, 0, 0" -5e+01) "None" true)
          (Rendering|Components|Light|SetIntensity (Variables|Default|GetPointLight) 0.0)
          (CallFunction|Spawnstairs))))))

(fn ConstructionScript)