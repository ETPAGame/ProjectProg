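; LoaderLvlB is a progression gate that opens a door once every target in CibleLvlA is dead.
; A looping timer polls the targets, folding their IsDead flags into Active, and a later tick acts on that result once.
; With Loader set, it opens Door and streams in Lvl_B without blocking; otherwise it only opens the door referenced by NewVar0.
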(event Custom|EventTock
  (if (Variables|Default|Getloader?)
    (if (Variables|Default|GetActive?)
      (Utilities|FlowControl|DoOnce false
        (:Completed
          (Default|OpenDoor (Variables|Default|GetDoor))
          (Class|GameplayStatics|LoadStreamLevelbySoftObjectPtr "/Game/Maps/lvl_B.lvl_B" true false)))
      (else
        (Variables|Default|SetActive? true)
        (for _array_element (Variables|Default|GetCibleLvlA)
          (Variables|Default|SetActive? (and (Variables|/Game/Blueprints/Cible.Cible_C|GetIsDead? _array_element) (Variables|Default|GetActive?))))))
    (elif (Variables|Default|GetActive?)
      (Utilities|FlowControl|DoOnce false
        (:Completed
          (Default|OpenDoor (Variables|Default|GetNewVar_0))))
      (else
        (Variables|Default|SetActive? true)
        (for _array_element_2 (Variables|Default|GetCibleLvlA)
          (Variables|Default|SetActive? (and (Variables|/Game/Blueprints/Cible.Cible_C|GetIsDead? _array_element_2) (Variables|Default|GetActive?))))))))

(event EventBeginPlay
  (Utilities|Time|SetTimerbyEvent (delegate Custom|EventTock) 2.5 true))

(fn ConstructionScript)