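; BP_Platform_Rotor is a rotating platform or bridge actor that swings on Toggle_Bridge and returns on Undo_Bridge.
; One of two timelines drives the angle, scaled by OverridePitch and offset 180 degrees when Reverse is set; the IsImpulse timeline automatically reverses after finishing.
; RotorX, RotorY and RotorZ select the root's world rotation axis, zeroing the others.
; The Y axis adds the current pitch on every update, unlike X and Z.
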(event Custom|Toggle_Bridge
  (bind _defaultsceneroot (Variables|Default|GetDefaultSceneRoot))
  (if (Variables|Default|GetReverse)
    (Variables|Default|SetReverse_Float 1.8e+02)
    (else
      (Variables|Default|SetReverse_Float 0.0)))
  (if (Variables|Default|GetisImpulse?)
    (bind _bridge_value (Timeline|Timeline_1 Play)
      (:Update
        (Variables|Default|SetBridgeVal (+ (* _bridge_value (Variables|Default|GetOverride%20Pitch)) (Variables|Default|GetReverse_Float)))
        (if (Variables|Default|GetRotorY?) :!label _label
          (Transformation|SetWorldRotation _defaultsceneroot (Math|Rotator|MakeRotator 0.0 (+ (Variables|Default|GetBridgeVal) (.pitch (Transformation|GetWorldRotation (Variables|Default|GetDefaultSceneRoot)))) 0.0) false false))
        (if (Variables|Default|GetRotorX?)
          (Transformation|SetWorldRotation _defaultsceneroot (Math|Rotator|MakeRotator (Variables|Default|GetBridgeVal) 0.0 0.0) false false))
        (if (Variables|Default|GetRotorZ?)
          (Transformation|SetWorldRotation _defaultsceneroot (Math|Rotator|MakeRotator 0.0 0.0 (Variables|Default|GetBridgeVal)) false false)))
      (:Finished
        (Timeline|Timeline_1 Reverse)))
    (else
      (bind _bridge_value_2 (Timeline|Timeline_0 Play)
        (:Update
          (Variables|Default|SetBridgeVal (+ (* _bridge_value_2 (Variables|Default|GetOverride%20Pitch)) (Variables|Default|GetReverse_Float)))
          (goto _label))))))

(event Custom|Undo_Bridge
  (bind _defaultsceneroot (Variables|Default|GetDefaultSceneRoot))
  (if (Variables|Default|GetReverse)
    (Variables|Default|SetReverse_Float 1.8e+02)
    (else
      (Variables|Default|SetReverse_Float 0.0)))
  (if (Variables|Default|GetisImpulse?)
    (bind _bridge_value (Timeline|Timeline_1 Reverse)
      (:Update
        (Variables|Default|SetBridgeVal (+ (* _bridge_value (Variables|Default|GetOverride%20Pitch)) (Variables|Default|GetReverse_Float)))
        (if (Variables|Default|GetRotorY?) :!label _label
          (Transformation|SetWorldRotation _defaultsceneroot (Math|Rotator|MakeRotator 0.0 (+ (Variables|Default|GetBridgeVal) (.pitch (Transformation|GetWorldRotation (Variables|Default|GetDefaultSceneRoot)))) 0.0) false false))
        (if (Variables|Default|GetRotorX?)
          (Transformation|SetWorldRotation _defaultsceneroot (Math|Rotator|MakeRotator (Variables|Default|GetBridgeVal) 0.0 0.0) false false))
        (if (Variables|Default|GetRotorZ?)
          (Transformation|SetWorldRotation _defaultsceneroot (Math|Rotator|MakeRotator 0.0 0.0 (Variables|Default|GetBridgeVal)) false false)))
      (:Finished
        (Timeline|Timeline_1 Reverse)))
    (else
      (bind _bridge_value_2 (Timeline|Timeline_0 Reverse)
        (:Update
          (Variables|Default|SetBridgeVal (+ (* _bridge_value_2 (Variables|Default|GetOverride%20Pitch)) (Variables|Default|GetReverse_Float)))
          (goto _label))))))

(event EventBeginPlay)

(event Collision|EventActorBeginOverlap
  (params (OtherActor :type Actor%20Object%20Reference)))

(event EventTick
  (params (DeltaSeconds :type Float%20%28single-precision%29)))

(fn ConstructionScript)