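; Platform_Rotor is a bridge or platform that tilts in pitch around its RotativePoint in response to impulse and occupancy events.
; ImpulseBridge runs a DoOnce-gated timeline that calls Reverse on finish, counting passes before restoring the starting rotation and resetting the gate.
; StayOnBridge plays a second timeline that tilts it only up to BlockAngle, and OutOfBridge reverses it.
; Both motions add an Override offset and scale by a Reverse multiplier.
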(event Custom|StayOnBridge
  (bind _bridge_value (Timeline|Timeline_1 Play)
    (:Update
      (if (not (> _bridge_value (Variables|Default|GetBlock%20Angle)))
        (Transformation|SetRelativeRotation (Variables|Default|GetRotative%20Point) (Math|Rotator|MakeRotator 0.0 (* (Variables|Default|GetReverse) (+ _bridge_value (Variables|Default|GetOverride))) 0.0) false false)))))

(event Custom|OutOfBridge
  (bind _bridge_value (Timeline|Timeline_1 Reverse)
    (:Update
      (if (not (> _bridge_value (Variables|Default|GetBlock%20Angle)))
        (Transformation|SetRelativeRotation (Variables|Default|GetRotative%20Point) (Math|Rotator|MakeRotator 0.0 (* (Variables|Default|GetReverse) (+ _bridge_value (Variables|Default|GetOverride))) 0.0) false false)))))

(event Custom|ImpulseBridge
  (bind _rotative_point (Variables|Default|GetRotative%20Point))
  (Utilities|FlowControl|DoOnce false :!label _label
    (:Completed
      (Variables|Default|SetPass 0)
      (Variables|Default|SetStarting%20Rotation (Variables|/Script/Engine.SceneComponent|GetRelativeRotation _rotative_point))
      (bind _newtrack_0 (Timeline|Timeline_0 Play)
        (:Update
          (Transformation|SetRelativeRotation _rotative_point (Math|Rotator|MakeRotator 0.0 (* (Variables|Default|GetReverse) (+ _newtrack_0 (Variables|Default|GetOverride))) 0.0) false false))
        (:Finished
          (if (> (Variables|Default|GetPass) 3)
            (Transformation|SetRelativeRotation _rotative_point (Variables|Default|GetStarting%20Rotation) false false)
            (goto _label Reset)
            (else
              (bind _result (Math|Integer|IncrementInt (Variables|Default|GetPass))
                (:%20%20
                  (Variables|Default|SetPass _result)
                  (Timeline|Timeline_0 Reverse))))))))))

(fn ConstructionScript)