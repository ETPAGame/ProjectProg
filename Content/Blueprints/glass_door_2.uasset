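; Glass door that toggles on CloseInteract; when flagged as ShootingRange, it responds only once every listed target is dead.
; A FlipFlop alternately plays and reverses a timeline.
; Each timeline update sets the root's relative location from its current world location plus a downward Z offset scaled by the track, so offsets accumulate.
; A DoOnce plays the door sound a single time at world origin.
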(event EventBeginPlay)

(event Collision|EventActorBeginOverlap
  (params (OtherActor :type Actor%20Object%20Reference)))

(event EventTick
  (params (DeltaSeconds :type Float%20%28single-precision%29)))

(event EventCloseInteract
  (params (Player :type First%20Person%20Character%20Object%20Reference))
  (bind _defaultsceneroot (Variables|Default|GetDefaultSceneRoot))
  (bind _listoftargets (Variables|Default|GetListOfTargets))
  (bind _returnvalue (Transformation|GetWorldLocation _defaultsceneroot))
  (if (Variables|Default|GetShootingRange?)
    (Variables|Default|SetokCount 0)
    (for _array_element _listoftargets
      (if (Variables|/Game/Blueprints/Cible.Cible_C|GetIsDead? _array_element)
        (bind _result (Math|Integer|IncrementInt (Variables|Default|GetokCount))
          (:%20%20
            (Variables|Default|SetokCount _result)))))
    (if (== (Variables|Default|GetokCount) (Utilities|Array|Length _listoftargets))
      (Utilities|FlowControl|FlipFlop :!label _label
        (:A
          (bind _newtrack_0 (Timeline|Timeline_0 Play)
            (:Update
              (Transformation|SetRelativeLocation _defaultsceneroot (Math|Vector|MakeVector (.x _returnvalue) (.y _returnvalue) (+ (* _newtrack_0 -4.9e+02) (.z _returnvalue))) false false)
              (Utilities|FlowControl|DoOnce false
                (:Completed
                  (Audio|PlaySoundatLocation "/Game/Son/glass_door.glass_door" "0, 0, 0" "0, 0, 0" 1.0 1.0 0.0 0 0 0))))))
        (:B
          (Timeline|Timeline_0 Reverse))))
    (else
      (goto _label))))

(fn ConstructionScript)