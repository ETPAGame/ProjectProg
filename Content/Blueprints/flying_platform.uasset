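; Moving platform that oscillates along a chosen X, Y or Z axis with configurable distance and speed.
; A Timeline moves the mesh and loops back and forth through a FlipFlop, after a start delay derived from world position.
; When linked to buttons or a target, it starts at zero scale.
; Tick restores full scale once both button lights are green or the target is down.
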(event Custom|LaunchPlatform
  (Components|Timeline|SetPlayRate (Variables|Default|GetTimeline_0) (Variables|Default|GetSpeed))
  (Utilities|FlowControl|FlipFlop
    (:A
      (bind _newtrack_0 (Timeline|Timeline_0 Play)
        (:Update
          (Transformation|SetRelativeLocation (Variables|Default|GetStaticMesh1) (Utilities|Select :Index (Variables|Default|GetDirection) :NewEnumerator0 (Math|Vector|MakeVector (* _newtrack_0 (* (Variables|Default|GetDistance) -1.0)) 0.0 0.0) :NewEnumerator1 (Math|Vector|MakeVector 0.0 (* _newtrack_0 (* (Variables|Default|GetDistance) -1.0)) 0.0) :NewEnumerator2 (Math|Vector|MakeVector 0.0 0.0 (* _newtrack_0 (* (Variables|Default|GetDistance) -1.0)))) false false))
        (:Finished
          (CallFunction|LaunchPlatform))))
    (:B
      (Timeline|Timeline_0 Reverse))))

(event Custom|Activ
  (Transformation|SetWorldScale3D (Variables|Default|GetScene) "1.000000,1.000000,1.000000"))

(event Collision|EventActorBeginOverlap
  (params (OtherActor :type Actor%20Object%20Reference)))

(event EventTick
  (params (DeltaSeconds :type Float%20%28single-precision%29))
  ;[1 1 1] Comment
  (if (or (Variables|Default|GetA%20bouton%20?) (Variables|Default|Getcible?))
    (bind _output_get (Variables|Default|SetActivate (or (and (== (Rendering|Components|Light|GetLightColor (Variables|/Game/Blueprints/Bouton.Bouton_C|GetPointLight (Variables|Default|GetBouton1))) "(R=0.000000,G=1.000000,B=0.000000,A=1.000000)") (== (Rendering|Components|Light|GetLightColor (Variables|/Game/Blueprints/Bouton.Bouton_C|GetPointLight (Variables|Default|GetBouton2))) "(R=0.000000,G=1.000000,B=0.000000,A=1.000000)")) (Variables|/Game/Blueprints/Cible.Cible_C|GetDOWN (Variables|Default|Getcible1)))))
    (if _output_get
      (Utilities|FlowControl|DoOnce false
        (:Completed
          (CallFunction|Activ))))))

(event EventBeginPlay
  (bind _staticmesh1 (Variables|Default|GetStaticMesh1))
  (bind _returnvalue (Transformation|GetWorldLocation _staticmesh1))
  (if (or (Variables|Default|GetA%20bouton%20?) (Variables|Default|Getcible?))
    (Transformation|SetWorldScale3D (Variables|Default|GetScene) "0, 0, 0")
    (Variables|Default|SetActivate false))
  (Utilities|FlowControl|Delay (Math|Float|Absolute(Float) (Math|Float|%(Float) (+ (.z _returnvalue) (.x _returnvalue) (.y _returnvalue)) 5.0)))
  (CallFunction|LaunchPlatform))

(fn ConstructionScript)