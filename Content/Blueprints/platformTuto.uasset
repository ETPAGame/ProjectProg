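; Tutorial platform actor, going by its name, that moves a static mesh along world X in a repeating timeline cycle.
; On BeginPlay it prints and waits a delay derived from the mesh's world Y modulo 5, staggering platforms by placement.
; Each timeline update adds the track value to current X, so travel accumulates per frame.
; On finish, a FlipFlop alternates reverse and forward playback.
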(event Custom|timeLine%20playing
  (bind _staticmesh (Variables|Default|GetStaticMesh))
  (bind _returnvalue (Transformation|GetWorldLocation _staticmesh))
  (Utilities|FlowControl|FlipFlop
    (:A
      (bind _newtrack_0 (Timeline|Timeline_0 ReverseFromEnd)
        (:Update
          (Transformation|SetWorldLocation _staticmesh (Math|Vector|MakeVector (+ (.x _returnvalue) _newtrack_0) (.y _returnvalue) (.z _returnvalue)) false false))
        (:Finished
          (CallFunction|TimeLinePlaying))))
    (:B
      (Timeline|Timeline_0 PlayFromStart))))

(event EventBeginPlay
  (bind _staticmesh (Variables|Default|GetStaticMesh))
  (bind _returnvalue (Transformation|GetWorldLocation _staticmesh))
  (bind _returnvalue_2 (Math|Float|%(Float) (.y _returnvalue) 5.0))
  (bind _returnvalue_3 (Math|Float|Absolute(Float) _returnvalue_2))
  (Development|PrintString (Utilities|String|ToString(Float) _returnvalue_3))
  (Utilities|FlowControl|Delay _returnvalue_3)
  (bind _newtrack_0 (Timeline|Timeline_0 Play)
    (:Update
      (Transformation|SetWorldLocation _staticmesh (Math|Vector|MakeVector (+ (.x _returnvalue) _newtrack_0) (.y _returnvalue) (.z _returnvalue)) false false))
    (:Finished
      (CallFunction|TimeLinePlaying))))

(event Collision|EventActorBeginOverlap
  (params (OtherActor :type Actor%20Object%20Reference)))

(event EventTick
  (params (DeltaSeconds :type Float%20%28single-precision%29)))

(fn ConstructionScript)