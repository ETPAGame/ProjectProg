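; PorteABoutonSol is a Blueprint that, by its name, is a door tied to floor buttons, though it currently only prints debug strings.
; Every Tick it treats a button as active when its PointLight color is pure green.
; With a valid Bouton2 it requires both buttons green and prints "2", otherwise it checks Bouton1 alone and prints "1".
; No door movement is implemented.
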(event EventBeginPlay)

(event Collision|EventActorBeginOverlap
  (params (OtherActor :type Actor%20Object%20Reference)))

(event EventTick
  (params (DeltaSeconds :type Float%20%28single-precision%29))
  (Utilities|IsValid (Variables|Default|GetBouton2)
    (:Is%20Valid
      (if (and (== (Rendering|Components|Light|GetLightColor (Variables|/Game/Blueprints/Bouton.Bouton_C|GetPointLight (Variables|Default|GetBouton1))) "(R=0.000000,G=1.000000,B=0.000000,A=1.000000)") (== (Rendering|Components|Light|GetLightColor (Variables|/Game/Blueprints/Bouton.Bouton_C|GetPointLight (Variables|Default|GetBouton2))) "(R=0.000000,G=1.000000,B=0.000000,A=1.000000)"))
        (Development|PrintString "2")))
    (:Is%20Not%20Valid
      (if (== (Rendering|Components|Light|GetLightColor (Variables|/Game/Blueprints/Bouton.Bouton_C|GetPointLight (Variables|Default|GetBouton1))) "(R=0.000000,G=1.000000,B=0.000000,A=1.000000)")
        (Development|PrintString "1")))))

(fn ConstructionScript)