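; Bouton is a pressure button that switches linked platforms while a Character stands in its capsule.
; Tick polls the capsule's overlaps and uses the Active flag to fire Activation or Deactivate only on a change.
; Both events recolor the point light and call Activation on every platform, while only pressing plays a sound.
; An optional RotorPlatform receives StayOnBridge on press and OutOfBridge on release.
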(event Custom|Activation
  (Audio|PlaySoundatLocation "/Game/Son/zone.zone" (Transformation|GetWorldLocation (Variables|Default|GetSphere)) "0, 0, 0" 1.0 1.0 0.0 0 0 0)
  (Rendering|Components|Light|SetLightColor (Variables|Default|GetPointLight) "(R=0.000000,G=1.000000,B=0.000000,A=1.000000)" true)
  (Variables|Default|SetActive? true)
  (Utilities|FlowControl|Sequence
    (:then_0
      (for _array_element (Variables|Default|GetPlatforms)
        (Default|Activation _array_element)))
    (:then_1
      (bind _rotor_platform (Variables|Default|GetRotor_Platform)
        (:then
          (Default|StayonBridge _rotor_platform))
        (:else)))))

(event Custom|Deactivate
  (Rendering|Components|Light|SetLightColor (Variables|Default|GetPointLight) "(R=1.000000,G=1.000000,B=1.000000,A=1.000000)" true)
  (Variables|Default|SetActive? false)
  (Utilities|FlowControl|Sequence
    (:then_0
      (for _array_element (Variables|Default|GetPlatforms)
        (Default|Activation _array_element)))
    (:then_1
      (bind _rotor_platform (Variables|Default|GetRotor_Platform)
        (:then
          (Default|OutOfBridge _rotor_platform))
        (:else)))))

(event EventBeginPlay)

(event Collision|EventActorBeginOverlap
  (params (OtherActor :type Actor%20Object%20Reference)))

(event EventTick
  (params (DeltaSeconds :type Float%20%28single-precision%29))
  (bind _active_ (Variables|Default|GetActive?))
  (if (> (Utilities|Array|Length (Collision|GetOverlappingActors (Variables|Default|GetCapsule) "/Script/Engine.Character" :!class /Script/Engine.PrimitiveComponent)) 0)
    (if (not _active_)
      (CallFunction|Activation))
    (elif _active_
      (CallFunction|Deactivate))))

(fn ConstructionScript)